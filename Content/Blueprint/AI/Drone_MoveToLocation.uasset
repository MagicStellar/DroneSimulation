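; Behavior tree task that directs the base drone toward the MoveToLocation blackboard vector.
; It fetches the drone from the game mode through an interface message and calls its move-to-location message with a fixed distance threshold.
; The returned bool is written inverted to the IsMoving blackboard key, and the task finishes successfully at once in either case.
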(event EventReceiveExecuteAI
  (params (OwnerController :type AI%20Controller%20Object%20Reference) (ControlledPawn :type Pawn%20Object%20Reference))
  (bind _basedrone (Class|BPIGameModeBase|BPIGetBaseDrone(Message) (Game|GetGameMode)))
  (bind _complete (Class|BPIDrone|BPIMovetoLocation(Message) _basedrone (Class|BTFunctionLibrary|GetBlackboardValueasVector (Variables|Default|GetMoveToLocation)) 1e+02))
  (if _complete
    (Class|BTFunctionLibrary|SetBlackboardValueasBool (Variables|Default|GetIsMoving) false)
    (else
      (Class|BTFunctionLibrary|SetBlackboardValueasBool (Variables|Default|GetIsMoving) true)))
  (AI|BehaviorTree|FinishExecute true))