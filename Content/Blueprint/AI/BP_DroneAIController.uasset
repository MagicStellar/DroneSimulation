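; AI controller for the drone that runs its behavior tree and switches it to chasing when it sees the player.
; On BeginPlay it registers with the game mode, starts BT_Drone and passes the blackboard component to the possessed BP_Drone.
; Perception updates filter for Player-tagged actors, handling stimuli as sight only for the first updated actor index.
; A successful stimulus stores locations and moves Patrol or Investigate to Chase, raising fly speed.
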(event OnPerceptionUpdated(AIPerception)
  (params (UpdatedActors :type Array%20of%20Actor%20Object%20References))
  ;[0 0 0] Check whether the character  is in zone
  (for (_array_element _array_index) UpdatedActors
    (if (Actor|ActorHasTag _array_element "Player")
      (bind _info (Class|AIPerceptionComponent|GetActorsPerception (Variables|Default|GetAIPerception) _array_element))
      (for _array_element_2 (.lastsensedstimuli _info)
        (Variables|Default|SetActiveSense _array_element_2)
        (switch int _array_index
          (:0
            (CallFunction|SightSense)))))))

(event Custom|SightSense
  (bind _activesense (Variables|Default|GetActiveSense))
  (bind (_age _expirationage _strength _stimuluslocation _receiverlocation _tag _bsuccessfullysensed) (Utilities|Struct|BreakAIStimulus _activesense))
  ;[0 0 0] Update On Character Sensed
  (if _bsuccessfullysensed
    (Development|PrintString "Player Sensed")
    (Variables|Default|SetPlayerLocation _stimuluslocation)
    (Variables|Default|SetDroneCurrentLocation _receiverlocation)
    (switch Utilities|FlowControl|Switch|SwitchonE_Drone_States (Variables|/Game/Blueprint/BP_Drone.BP_Drone_C|GetDroneAIState (Variables|Default|GetBP_Drone))
      (:NewEnumerator0
        _)
      (:NewEnumerator3
        _))
    (Variables|/Game/Blueprint/BP_Drone.BP_Drone_C|SetDroneAIState (Variables|Default|GetBP_Drone) "NewEnumerator1")
    (Variables|/Script/Engine.CharacterMovementComponent|SetMaxFlySpeed (Variables|/Script/Engine.Character|GetCharacterMovement (Variables|Default|GetBP_Drone)) 8e+02)
    (else
      (Development|PrintString "Player out of Sight"))))

(event EventBeginPlay
  ;[0.02372 1 0.3523] BeginPlay
  (Class|BPIGameModeBase|BPISetAIDroneController(Message) (Game|GetGameMode) self)
  (AI|RunBehaviorTree "/Game/Blueprint/AI/BT_Drone.BT_Drone")
  (bind _asbp_drone (Utilities|Casting|CastToBP_Drone (Pawn|GetControlledPawn))
    (:then
      (Variables|Default|SetBP_Drone _asbp_drone)
      (Variables|/Game/Blueprint/BP_Drone.BP_Drone_C|SetBlackboard%20Component (Variables|Default|GetBP_Drone) (Variables|Default|Getcurrentblackboard)))
    (:CastFailed
      (Development|PrintString "cast failed"))))

(fn ConstructionScript)