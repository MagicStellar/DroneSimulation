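; Game mode Blueprint that acts as a shared registry for key actor references in the game.
; It stores the AI drone controller, base drone, player one and a third-person character through setter events, with matching getter functions returning each.
; The BPI naming suggests access through a Blueprint Interface, letting other Blueprints share references via the game mode.
; It contains no gameplay logic of its own.
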(event EventBeginPlay)

(event EventTick
  (params (DeltaSeconds :type Float%20%28single-precision%29)))

(event EventBPISetAIDroneController
  (params (AIDroneController :type BP%20Drone%20AI%20Controller%20Object%20Reference))
  (Variables|Default|SetAIDrone%20Controller AIDroneController))

(event EventBPISetPlayerOne
  (params (ThirdPersonCharacter :type BP%20Third%20Person%20Character%20Object%20Reference))
  (Variables|Default|SetPlayerOne ThirdPersonCharacter))

(event EventBPISetBaseDrone
  (params (BpDrone :type BP%20Drone%20Object%20Reference))
  (Variables|Default|SetBp%20Drone BpDrone))

(event EventSetTPP
  (params (ThirdPersonCharacter :type BP%20Third%20Person%20Character%20Object%20Reference))
  (Variables|Default|SetThird%20Person%20Character ThirdPersonCharacter))

(fn ConstructionScript)

(fn BPIGetAIDroneController
  (return (Variables|Default|GetAIDrone%20Controller)))

(fn BPIGetBaseDrone
  (return (Variables|Default|GetBp%20Drone)))

(fn BPIGetPlayerOne
  (return (Variables|Default|GetPlayerOne)))

(fn GetTPP
  (return (Variables|Default|GetThird%20Person%20Character)))